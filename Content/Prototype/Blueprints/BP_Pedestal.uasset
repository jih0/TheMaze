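; BP_Pedestal is a riddle pedestal that shows a tooltip when the player enters its collision box and reveals the riddle on E.
; Once the riddle is attempted, keys 1 to 3 answer it, with 2 correct and the others wrong.
; Tick yaws the text roots toward the player and polls the result flags to show win or lose text and disable input.
; Leaving hides riddle and tooltip but keeps input enabled and rotation on.
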(event OnComponentBeginOverlap(Collision_Box)
  (params (OtherActor :type Actor%20Object%20Reference) (OtherComp :type Primitive%20Component%20Object%20Reference) (OtherBodyIndex :type Integer) (bFromSweep :type Boolean) (SweepResult :type Hit%20Result%20Structure%20%28by%20ref%29))
  ;[1 1 1] On Collision Box Enter
  (if (== OtherActor (Game|GetPlayerCharacter 0))
    (Utilities|FlowControl|Sequence
      (:then_0
        (Variables|Default|SetbRotate_Text true))
      (:then_1
        (Input|EnableInput (Game|GetPlayerController 0)))
      (:then_2
        (Development|SetHiddeninGame (Variables|Default|GetTooltip) false false)))))

(event OnComponentEndOverlap(Collision_Box)
  (params (OtherActor :type Actor%20Object%20Reference) (OtherComp :type Primitive%20Component%20Object%20Reference) (OtherBodyIndex :type Integer))
  ;[1 1 1] On Collision Box Enter
  (if (== OtherActor (Game|GetPlayerCharacter 0))
    (Variables|Default|SetbRotate_Text false)
    (Utilities|FlowControl|Sequence
      (:then_0
        (Variables|Default|SetbRotate_Text true))
      (:then_1
        (Development|SetHiddeninGame (Variables|Default|GetRiddle_Text_Root) true true))
      (:then_2
        (Development|SetHiddeninGame (Variables|Default|GetTooltip) true false)))))

(event EventTick
  (params (DeltaSeconds :type Float%20%28single-precision%29))
  (bind _returnvalue (Game|GetPlayerController 0))
  ;[1 1 1] Text Rotation
  (Utilities|FlowControl|Sequence
    (:then_0
      (if (Variables|Default|GetbRotate_Text)
        (Transformation|SetWorldRotation (Variables|Default|GetWinLose_Text_Root) (Math|Rotator|MakeRotator (.Roll (Math|Rotator|BreakRotator (Transformation|GetWorldRotation (Variables|Default|GetWinLose_Text_Root)))) 0.0 (.Yaw (Math|Rotator|BreakRotator (Math|Rotator|FindLookatRotation (Transformation|GetWorldLocation (Variables|Default|GetWinLose_Text_Root)) (Transformation|GetActorLocation (Game|GetPlayerCharacter 0)))))) false false)))
    (:then_1
      (if (Variables|Default|GetbRotate_Text)
        (Transformation|SetWorldRotation (Variables|Default|GetRiddle_Text_Root) (Math|Rotator|MakeRotator (.Roll (Math|Rotator|BreakRotator (Transformation|GetWorldRotation (Variables|Default|GetRiddle_Text_Root)))) 0.0 (.Yaw (Math|Rotator|BreakRotator (Math|Rotator|FindLookatRotation (Transformation|GetWorldLocation (Variables|Default|GetRiddle_Text_Root)) (Transformation|GetActorLocation (Game|GetPlayerCharacter 0)))))) false false)))
    (:then_2
      ;[1 1 1] Win?Lose Check and Result
      (Utilities|FlowControl|Sequence
        (:then_0
          (if (Variables|Default|GetbCorrect)
            (Utilities|FlowControl|Sequence
              (:then_0
                (Development|SetHiddeninGame (Variables|Default|GetRiddle_Text_Root) true true))
              (:then_1
                (Development|SetHiddeninGame (Variables|Default|GetWin_Text) false false))
              (:then_2
                (Input|DisableInput _returnvalue)))))
        (:then_1
          (if (Variables|Default|GetbFalse)
            (Utilities|FlowControl|Sequence
              (:then_0
                (Development|SetHiddeninGame (Variables|Default|GetRiddle_Text_Root) true true))
              (:then_1
                (Development|SetHiddeninGame (Variables|Default|GetLose_Text) false false))
              (:then_2
                (Input|DisableInput _returnvalue)))))))))

(event Input|KeyboardEvents|E
  (params (Key :type Key%20Structure :default "AnyKey"))
  ;[1 1 1] On Collision Box Enter
  (:Pressed
    (Development|SetHiddeninGame (Variables|Default|GetRiddle_Text_Root) false true)
    (Variables|Default|SetbRiddleAttempted true)))

(event Input|KeyboardEvents|1
  (params (Key :type Key%20Structure :default "AnyKey"))
  ;[1 1 1] Win?Lose Check and Result
  (:Pressed
    (if (Variables|Default|GetbRiddleAttempted)
      (Variables|Default|SetbFalse true))))

(event Input|KeyboardEvents|2
  (params (Key :type Key%20Structure :default "AnyKey"))
  ;[1 1 1] Win?Lose Check and Result
  (:Pressed
    (if (Variables|Default|GetbRiddleAttempted)
      (Variables|Default|SetbCorrect true))))

(event Input|KeyboardEvents|3
  (params (Key :type Key%20Structure :default "AnyKey"))
  ;[1 1 1] Win?Lose Check and Result
  (:Pressed
    (if (Variables|Default|GetbRiddleAttempted)
      (Variables|Default|SetbFalse true))))

(fn ConstructionScript)